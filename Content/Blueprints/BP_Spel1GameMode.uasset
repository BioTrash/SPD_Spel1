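; Game mode for Spel1 that handles loading and respawning the player and advancing enemy waves.
; Respawn resets health pickups, slime drops, spawn zones and boss, restores the player from the save slot, fades out level music, then saves.
; BeginPlay caches health pickups and, outside debug mode, runs the same sequence minus the pickup reset.
; CheckEnemyLeft increments the wave and calls the next spawn once no enemies remain.
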(event `Update Slime Ammo`
  ;[1 1 1] Update Slime Ammo (Jeremy)
  (`/Game/Blueprints/BP_PlayerCharacter.Set Slime Ammo` (`self.Player`)))

(event `Reset Player transform`
  (params (IsNewGame :type Boolean :default false) (SaveFile :type "/Game/Jeremy/Blueprints/BP_SaveGame Object Reference"))
  (bind _returnvalue (`GameplayStatics.GetPlayerPawn` 0))
  ;[1 1 1] Reset Player Transform (Jeremy)
  (if IsNewGame
    (set `/Game/Jeremy/Blueprints/BP_SaveGame.PlayerPos` (`self.GetTransform` (`self.K2_FindPlayerStart` null)) SaveFile))
  (`self.K2_SetActorTransform` _returnvalue (`/Game/Jeremy/Blueprints/BP_SaveGame.PlayerPos` SaveFile) false false)
  (bind _asbp_player_character (cast `/Game/Blueprints/BP_PlayerCharacter` _returnvalue))
  (set `self.Player` _asbp_player_character))

(event `Update Health`
  (bind _player (`self.Player`))
  ;[1 1 1] Update Health (Jeremy)
  (`/Game/Blueprints/BP_PlayerCharacter.Increase Health` _player (`PlayerCharacter.MaxHealth` _player)))

(event `Respawn Player`
  ;[1 1 1] Load Game / Respawn Player (Jeremy)
  (`self.Reset HP Pickups`)
  (`self.Remove slime drops` :!label _label)
  (`self.Reset Spawnzones`)
  (`self.Reset Boss`)
  (bind _returnvalue (`GameplayStatics.LoadGameFromSlot` (`self.SaveName`)))
  (bind _asbp_save_game (cast `/Game/Jeremy/Blueprints/BP_SaveGame` _returnvalue))
  (bind _output_get (set `self.SaveFile` _asbp_save_game))
  (`self.Reset Player transform` (`/Game/Jeremy/Blueprints/BP_SaveGame.IsNewGame` _output_get) _output_get)
  (`self.Update Health`)
  (`self.Update Slime Ammo`)
  (`/Game/Blueprints/BP_PlayerCharacter.Reset Player` (`self.Player`))
  (bind _returnvalue_2 (`GameplayStatics.GetActorOfClass` "/Game/Jeremy/Blueprints/BP_MusicManager.BP_MusicManager_C"))
  (bind _level1_music (`/Game/Jeremy/Blueprints/BP_MusicManager.Level1_Music` _returnvalue_2))
  (`AudioComponent.FadeOut` _level1_music 2.0 0.0 "Linear")
  (`AudioComponent.SetPaused` _level1_music true)
  (`GameplayStatics.SaveGameToSlot` (`self.SaveFile`) (`self.SaveName`)))

(event `self.ReceiveBeginPlay`
  ;[1 1 1] Load Game / Respawn Player (Jeremy)
  (`self.Find HP Pickups`)
  (if (not (`self.DebugMode`))
    (goto _label)))

(event `Check Enemy Left`
  ;[1 1 1] When a enemy dies check how many are left. If all are dead spawn next wave (Jeremy)
  (if (<= (`self.EnemiesAlive`) 0)
    (bind _result (`/Engine/EditorBlueprintResources/StandardMacros.IncrementInt` (`self.WaveCount`))
      (:`  `
        (set `self.WaveCount` _result)
        (`self.SpawnNextWave`)))))

(event `Reset Spawnzones`
  ;[1 1 1] Reset Spawnzones (Jeremy)
  (bind _outactors (`GameplayStatics.GetAllActorsOfClass` "/Game/Jeremy/Blueprints/BP_SpawnzoneEnemy.BP_SpawnzoneEnemy_C"))
  (for _array_element _outactors
    (`/Game/Jeremy/Blueprints/BP_SpawnzoneEnemy.Reset Spawnzone` _array_element)
    (set `self.WaveCount` 1)
    (set `self.EnemiesAlive` 0)))

(event `Reset Boss`
  ;[1 1 1] Reset the Boss (Jeremy)
  (bind _returnvalue (`GameplayStatics.GetActorOfClass` "/Game/AI/EnemyAI/Bosses/BossFirstLevel/BP_SlimeBossAI.BP_SlimeBossAI_C"))
  (bind _asbp_slime_boss_ai (cast `/Game/AI/EnemyAI/Bosses/BossFirstLevel/BP_SlimeBossAI` _returnvalue))
  (`/Game/AI/EnemyAI/Bosses/BossFirstLevel/BP_SlimeBossAI.Reset Boss` _asbp_slime_boss_ai))

(event `Remove slime drops`
  ;[1 1 1] Remove slime drops (Jeremy)
  (bind _outactors (`GameplayStatics.GetAllActorsOfClass` "/Game/Blueprints/BP_SlimePickUp.BP_SlimePickUp_C"))
  (for _array_element _outactors
    (`self.K2_DestroyActor` _array_element)))

(event `Find HP Pickups`
  ;[1 1 1] Find HP pickups (Jeremy)
  (bind _outactors (`GameplayStatics.GetAllActorsOfClass` "/Game/Blueprints/BP_HealthPickUp.BP_HealthPickUp_C"))
  (set `self.HealthPickups` _outactors))

(event `Reset HP Pickups`
  ;[1 1 1] Reset HP pickups (Jeremy)
  (if (`KismetArrayLibrary.Array_IsNotEmpty` (`self.HealthPickups`))
    (for _array_element (`self.HealthPickups`)
      (bind _asbp_health_pick_up (cast `/Game/Blueprints/BP_HealthPickUp` _array_element))
      (`/Game/Blueprints/BP_HealthPickUp.Reset HP` _asbp_health_pick_up))))

(fn `UserConstructionScript`)