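; BP_Slime is a slime ammo pickup that flies toward the player who overlaps its trigger.
; It reacts only when the player's trigger weapon has an alternative fire mode with slime ammo below maximum.
; A Timeline lerps the mesh toward the player, and a short Delay inside its Update then calls SlimePickUp with the current ammo, plays a sound and destroys the actor.
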(event `self.Trigger.OnComponentBeginOverlap`
  (params (OverlappedComponent :type "PrimitiveComponent Object Reference") (OtherActor :type "Actor Object Reference") (OtherComp :type "PrimitiveComponent Object Reference") (OtherBodyIndex :type Integer) (bFromSweep :type Boolean) (SweepResult :type "HitResult Structure (by ref)"))
  (if (`self.ActorHasTag` OtherActor "Player")
    (bind _asbp_player_character (cast `/Game/Blueprints/BP_PlayerCharacter` OtherActor))
    (bind _asnon_projectile_weapon (cast `NonProjectileWeapon` (`PlayerCharacter.GetTriggerWeapon` _asbp_player_character)))
    (bind _asalternative_fire_mode (cast `AlternativeFireMode` _asnon_projectile_weapon))
    (bind _returnvalue (`AlternativeFireMode.GetCurrentSlimeAmmo` _asalternative_fire_mode))
    (if (< _returnvalue (`AlternativeFireMode.MaxSlimeAmmo` _asalternative_fire_mode))
      (bind (_direction _newtrack_0) (`Timeline|Timeline`)
        (:`Update`
          (`SceneComponent.K2_SetWorldLocation` (`self.SlimeMesh`) (`KismetMathLibrary.VLerp` (`SceneComponent.K2_GetComponentLocation` (`self.SlimeMesh`)) (`self.K2_GetActorLocation` _asbp_player_character) _newtrack_0) false false)
          (`KismetSystemLibrary.Delay` 0.1)
          (`/Game/Blueprints/BP_PlayerCharacter.Slime Pick Up` _asbp_player_character _returnvalue)
          (`GameplayStatics.PlaySoundAtLocation` "/Engine/VREditor/Sounds/UI/Dockable_Window_Pick_Up.Dockable_Window_Pick_Up" (`self.K2_GetActorLocation`) (struct) 1.0 1.0 0.0 null null null null)
          (`self.K2_DestroyActor`))))))

(fn `UserConstructionScript`)