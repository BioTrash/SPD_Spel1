(event Custom|Increase%20Health
  (params (New%20Health :type Float%20%28double-precision%29))
  ;[1 1 1] Increase Health Pick Up
  (Variables|Default|SetHealth (+ (Variables|Default|GetHealth) New%20Health))
  (if (> (Variables|Default|GetHealth) 1e+02)
    (Variables|Default|SetHealth 1e+02)))

(event EventDestroyed
  ;[1 1 1] Destroy weapon
  (bind _returnvalue (Actor|GetActorOfClass "/Game/Blueprints/BP_TestWeapon.BP_TestWeapon_C"))
  (Actor|DestroyActor _returnvalue))

(event EventBeginPlay
  ;[1 1 1] Show Health Widget and Dash cooldown
  (bind _returnvalue (UserInterface|CreateWidget "/Game/UI/WBP_DashCooldown.WBP_DashCooldown_C"))
  (bind _returnvalue_2 (UserInterface|CreateWidget "/Game/UI/WBP_Health.WBP_Health_C"))
  (UserInterface|Viewport|AddtoViewport _returnvalue_2 0))

(event EventTick
  (params (DeltaSeconds :type Float%20%28single-precision%29))
  (bind _returnvalue (Game|GetPlayerController 0))
  (if (<= (Class|PlayerCharacter|GetHealthPercent) 0.0)
    (Utilities|FlowControl|DoOnce false
      (:Completed
        (Utilities|Casting|CastToBP_Spel1GameMode (Game|GetGameMode))
        (bind _returnvalue_2 (UserInterface|CreateWidget "/Game/Jeremy/Widgets/WBP_YouLost.WBP_YouLost_C"))
        (UserInterface|Viewport|AddtoViewport _returnvalue_2 0)
        (Variables|/Script/Engine.PlayerController|SetbShowMouseCursor _returnvalue true)
        (Input|SetInputModeUIOnly _returnvalue _returnvalue_2 "DoNotLock" false)))))

(event Input|ActionEvents|InputActionDash
  (params (Key :type Key%20Structure :default "None"))
  ;[1 1 1] Dash Cooldown
  (:Pressed
    (if (Variables|Default|GetCanDash?)
      (Class|PlayerCharacter|Dash)
      (Variables|Default|SetCanDash? false)
      (Utilities|FlowControl|Delay 3.0)
      (Variables|Default|SetCanDash? true))))

(event Input|KeyboardEvents|DebugKey1
  (params (Key :type Key%20Structure :default "None") (ActionValue :type Input%20Action%20Value%20Structure))
  (bind _returnvalue (Game|GetPlayerController 0))
  (:Pressed
    (Utilities|FlowControl|DoOnce false
      (:Completed
        (Utilities|Casting|CastToBP_Spel1GameMode (Game|GetGameMode))
        (bind _returnvalue_2 (UserInterface|CreateWidget "/Game/Jeremy/Widgets/WBP_YouLost.WBP_YouLost_C"))
        (UserInterface|Viewport|AddtoViewport _returnvalue_2 0)
        (Variables|/Script/Engine.PlayerController|SetbShowMouseCursor _returnvalue true)
        (Input|SetInputModeUIOnly _returnvalue _returnvalue_2 "DoNotLock" false)))))

(event Input|KeyboardEvents|E
  (params (Key :type Key%20Structure :default "None"))
  ;[1 1 1] Press button for door
  (:Pressed
    (bind _array_element (Utilities|Array|ForEachLoopwithBreak (Collision|GetOverlappingActors "/Game/Blueprints/BP_Button.BP_Button_C" :!class /Script/Engine.Actor) :!label _label)
      (:LoopBody
        (if (Utilities|DoesObjectImplementInterface _array_element "/Game/Blueprints/BP_InteractInterface.BP_InteractInterface_C")
          (Class|BPInteractInterface|Interact(Message) _array_element self)
          (goto _label Break))))))

(event Input|KeyboardEvents|P
  (params (Key :type Key%20Structure :default "None"))
  (bind _returnvalue (Game|GetPlayerController 0))
  ;[1 1 1] Pause menu
  (:Pressed
    (bind _returnvalue_2 (UserInterface|CreateWidget "/Game/Jeremy/Widgets/WBP_PauseMenu.WBP_PauseMenu_C"))
    (UserInterface|Viewport|AddtoViewport _returnvalue_2 0)
    (Variables|/Script/Engine.PlayerController|SetbShowMouseCursor _returnvalue true)
    (Input|SetInputModeUIOnly _returnvalue _returnvalue_2 "DoNotLock" false)))

(fn ConstructionScript)