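; BP_RushEnemy is a slime enemy that reports itself to BP_Spel1GameMode's live enemy count.
; It increments EnemiesAlive on spawn, then on death plays a sound, decrements the count and calls CheckEnemyLeft.
; Death always spawns a BP_SlimePickUp, as the random-roll branch has no effect and a random number is printed for debugging.
; Taking any damage activates its Hit component.
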(event `self.ReceiveBeginPlay`
  ;[1 1 1] Increase "Enemies Alive" in the game mode when enemy spawns.
  (bind _asbp_spel_1game_mode (cast `/Game/Blueprints/BP_Spel1GameMode` (`GameplayStatics.GetGameMode`)))
  (`/Engine/EditorBlueprintResources/StandardMacros.IncrementInt` (`/Game/Blueprints/BP_Spel1GameMode.EnemiesAlive` _asbp_spel_1game_mode)))

(event `self.OnEnemyDeath`
  (bind _returnvalue (`KismetMathLibrary.RandomFloatInRange` 0.0 1.0))
  ;[1 1 1] Decrease "Enemies Alive" in the game mode when enemy dies and check how many enemies are left
  (`GameplayStatics.PlaySoundAtLocation` "/Game/Music/SoundEffects/Cues/SlimeDeath.SlimeDeath" (`self.K2_GetActorLocation`) (struct) 1.0 1.0 0.0 null null null null)
  (bind _asbp_spel_1game_mode (cast `/Game/Blueprints/BP_Spel1GameMode` (`GameplayStatics.GetGameMode`)))
  (`/Engine/EditorBlueprintResources/StandardMacros.DecrementInt` (`/Game/Blueprints/BP_Spel1GameMode.EnemiesAlive` _asbp_spel_1game_mode)
    (:`  `
      (if (>= _returnvalue 0.33)
        _
        (else
          _))
      (`KismetSystemLibrary.PrintText` (`KismetTextLibrary.Conv_DoubleToText` _returnvalue "HalfToEven"))
      (`|SpawnActorFromClass` "/Game/Blueprints/BP_SlimePickUp.BP_SlimePickUp_C" (`self.GetTransform`) "AdjustIfPossibleButAlwaysSpawn" "MultiplyWithRoot" null null)
      (`/Game/Blueprints/BP_Spel1GameMode.Check Enemy Left` _asbp_spel_1game_mode))))

(event `self.ReceiveAnyDamage`
  (params (Damage :type "Float (single-precision)") (DamageType :type "DamageType Object Reference") (InstigatedBy :type "Controller Object Reference") (DamageCauser :type "Actor Object Reference"))
  (`ActorComponent.Activate` (`self.Hit`) false))

(fn `UserConstructionScript`)