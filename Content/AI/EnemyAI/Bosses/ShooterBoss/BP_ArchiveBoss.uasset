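; BP_ArchiveBoss is a shooter boss enemy that registers itself with BP_Spel1GameMode's count of living enemies.
; It increments EnemiesAlive on BeginPlay.
; On death it plays a 2D splat sound, decrements the count and has the game mode check how many enemies remain.
; Any damage taken activates its TakeDamageEffect for hit feedback.
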(event `self.ReceiveBeginPlay`
  ;[1 1 1] Increase "Enemies Alive" in the game mode when enemy spawns.
  (bind _asbp_spel_1game_mode (cast `/Game/Blueprints/BP_Spel1GameMode` (`GameplayStatics.GetGameMode`)))
  (`/Engine/EditorBlueprintResources/StandardMacros.IncrementInt` (`/Game/Blueprints/BP_Spel1GameMode.EnemiesAlive` _asbp_spel_1game_mode)))

(event `self.OnEnemyDeath`
  ;[1 1 1] Decrease "Enemies Alive" in the game mode when enemy dies and check how many enemies are left
  (`GameplayStatics.PlaySound2D` "/Game/Music/SoundEffects/Splatter/impactsplat02_mp3.impactsplat02_mp3" 1.0 1.0 0.0 null null)
  (bind _asbp_spel_1game_mode (cast `/Game/Blueprints/BP_Spel1GameMode` (`GameplayStatics.GetGameMode`)))
  (`/Engine/EditorBlueprintResources/StandardMacros.DecrementInt` (`/Game/Blueprints/BP_Spel1GameMode.EnemiesAlive` _asbp_spel_1game_mode)
    (:`  `
      (`/Game/Blueprints/BP_Spel1GameMode.Check Enemy Left` _asbp_spel_1game_mode))))

(event `self.ReceiveAnyDamage`
  (params (Damage :type "Float (single-precision)") (DamageType :type "DamageType Object Reference") (InstigatedBy :type "Controller Object Reference") (DamageCauser :type "Actor Object Reference"))
  (`ActorComponent.Activate` (`self.TakeDamageEffect`) false))

(fn `UserConstructionScript`)