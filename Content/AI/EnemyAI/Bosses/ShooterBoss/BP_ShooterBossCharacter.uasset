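; Shooter boss character that stays dormant until its spawn effect finishes, then activates for the fight.
; BeginPlay disables controller tick and collision; the effect's completion, guarded by a resettable DoOnce, re-enables both, reveals the mesh and creates the boss health widget.
; ResetBoss restores health and dormancy, removes the widget, resets the room trigger and re-arms the DoOnce.
; Death removes the health widget; weapon visibility calls are left unconnected.
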(event `self.Spawn Effect.OnSystemFinished`
  (params (PSystem :type "NiagaraComponent Object Reference"))
  ;[1 1 1] Activate tick and show boss when spawn effect is finished
  (`/Engine/EditorBlueprintResources/StandardMacros.DoOnce` false :!label _label
    (:`Completed`
      (`self.SetActorTickEnabled` (`self.GetController`) true)
      (`SceneComponent.SetHiddenInGame` (`self.Mesh`) false false)
      (`self.SetActorEnableCollision` true)
      (bind _returnvalue (`|CreateWidget` "/Game/UI/WBP_BossHealth2.WBP_BossHealth2_C"))
      (`UserWidget.AddToViewport` _returnvalue 0))))

(event `Reset Boss`
  ;[1 1 1] Reset
  (`|ExecutionSequence`
    (:`then_0`
      (`self.ResetHealth`)
      (`self.SetActorTickEnabled` (`self.GetController`) false)
      (`SceneComponent.SetHiddenInGame` (`self.Mesh`) true false)
      (`self.SetActorEnableCollision` false)
      (bind _foundwidgets (`WidgetBlueprintLibrary.GetAllWidgetsOfClass` "/Game/UI/WBP_BossHealth2.WBP_BossHealth2_C"))
      (`Widget.RemoveFromParent` _foundwidgets)
      (bind _asbp_boss_room_trigger (cast `/Game/Jeremy/Blueprints/BP_BossRoomTrigger` (`self.BossRoomTrigger`)))
      (`/Game/Jeremy/Blueprints/BP_BossRoomTrigger.Reset` _asbp_boss_room_trigger))
    (:`then_1`
      (goto _label :!via `Reset`))))

(event `self.ReceiveBeginPlay`
  ;[1 1 1] Disable Tick and hide weapon
  (`self.SetActorTickEnabled` (`self.GetController`) false)
  (`self.SetActorEnableCollision` false))

(event `self.OnEnemyDeath`
  ;[1 1 1] Boss Death
  (bind _foundwidgets (`WidgetBlueprintLibrary.GetAllWidgetsOfClass` "/Game/UI/WBP_BossHealth2.WBP_BossHealth2_C"))
  (`Widget.RemoveFromParent` _foundwidgets))

(fn `UserConstructionScript`)