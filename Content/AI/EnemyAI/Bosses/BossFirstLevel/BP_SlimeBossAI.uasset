(event `self.Spawn Effect.OnSystemFinished`
  (params (PSystem :type "NiagaraComponent Object Reference"))
  ;[1 1 1] Activate tick and show boss when spawn effect is finished
  (`/Engine/EditorBlueprintResources/StandardMacros.DoOnce` false :!label _label
    (:`Completed`
      (`self.SetActorTickEnabled` (`self.GetController`) true)
      (`SceneComponent.SetHiddenInGame` (`self.HeadMesh`) false false)
      (bind _returnvalue (`|CreateWidget` "/Game/Jeremy/Widgets/WBP_BossHealth.WBP_BossHealth_C"))
      (`UserWidget.AddToViewport` _returnvalue 0))))

(event `self.ReceiveBeginPlay`
  ;[1 1 1] Disable Tick
  (`self.SetActorTickEnabled` (`self.GetController`) false))

(event `self.ReceiveTick`
  (params (DeltaSeconds :type "Float (single-precision)"))
  ;[1 1 1] Death + You Win
  (if (<= (`self.GetHealth`) 0.0)
    (bind _returnvalue (`|CreateWidget` "/Game/Jeremy/Widgets/WBP_YouWin.WBP_YouWin_C"))
    (`UserWidget.AddToViewport` _returnvalue 0)))

(event `Reset Boss`
  ;[1 1 1] Reset
  (`self.ResetHealth`)
  (`self.SetActorTickEnabled` (`self.GetController`) false)
  (`SceneComponent.SetHiddenInGame` (`self.HeadMesh`) true false)
  (bind _asbp_boss_room_trigger (cast `/Game/Jeremy/Blueprints/BP_BossRoomTrigger` (`self.BossRoomTrigger`)))
  (`/Game/Jeremy/Blueprints/BP_BossRoomTrigger.Reset` _asbp_boss_room_trigger)
  (goto _label :!via `Reset`))

(fn `UserConstructionScript`)