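; BP_RushEnemy is an enemy that reports its death to the spawn zone it spawned in.
; On overlap it caches the overlapped BP_SpawnzoneEnemy as its Spawnzone.
; On death it decrements that zone's EnemiesAlive count, prints it for debugging, and calls CheckEnemyLeft on the zone.
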(event `self.OnEnemyDeath`
  (bind _spawnzone (`self.Spawnzone`))
  ;[1 1 1] Death, when enemy dies enemies count inside spawnzone updates.
  (bind _result (`/Engine/EditorBlueprintResources/StandardMacros.DecrementInt` (`/Game/Jeremy/Blueprints/BP_SpawnzoneEnemy.EnemiesAlive` _spawnzone))
    (:`  `
      (bind _output_get (set `/Game/Jeremy/Blueprints/BP_SpawnzoneEnemy.EnemiesAlive` _result _spawnzone))
      (`KismetSystemLibrary.PrintString` (`KismetStringLibrary.Conv_IntToString` _output_get))
      (`/Game/Jeremy/Blueprints/BP_SpawnzoneEnemy.CheckEnemyLeft` _spawnzone))))

(event `self.ReceiveActorBeginOverlap`
  (params (OtherActor :type "Actor Object Reference"))
  ;[1 1 1] Get the spawnzone the enemy spawned inside.
  (bind _asbp_spawnzone_enemy (cast `/Game/Jeremy/Blueprints/BP_SpawnzoneEnemy` OtherActor))
  (set `self.Spawnzone` _asbp_spawnzone_enemy))

(fn `UserConstructionScript`)