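; BP_AIFlyingEnemy is an enemy that chases and attacks the player once PawnSensing spots a pawn.
; Each sighting sets IsSeeingPlayer and runs FollowPlayer, which re-enables CanAttack and uses AIMoveTo toward player 0.
; On arrival it plays an attack montage, waits out its length and prints "Damage" without applying any.
; Tick halts movement until the first sighting; the seeing flag is effectively never cleared afterwards.
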(event `self.ReceiveTick`
  (params (DeltaSeconds :type "Float (single-precision)"))
  (if (not (`self.isSeeingPlayer?`))
    (`MovementComponent.StopMovementImmediately` (`self.CharacterMovement`))))

(event `self.PawnSensing.OnSeePawn`
  (params (Pawn :type "Pawn Object Reference"))
  (set `self.isSeeingPlayer?` true)
  (`self.FollowPlayer`))

(event `FollowPlayer`
  (set `self.CanAttack` true)
  (if (`self.isSeeingPlayer?`)
    (`|AIMoveTo` self (0.0 0.0 0.0) (`GameplayStatics.GetPlayerCharacter` 0) 20.0
      (:`OnSuccess`
        (if (`self.CanAttack`)
          (set `self.CanAttack` false)
          (bind _returnvalue (`self.PlayAnimMontage` "/Game/TestEnemy/Wraith/Animations/Ability_R_Montage.Ability_R_Montage"))
          (`KismetSystemLibrary.Delay` _returnvalue)
          (set `self.CanAttack` true)
          (`KismetSystemLibrary.PrintString` "Damage"))))
    (else
      (set `self.isSeeingPlayer?` false))))

(fn `UserConstructionScript`)