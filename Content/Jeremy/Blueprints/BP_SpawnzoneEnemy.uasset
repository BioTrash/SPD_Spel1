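; Enemy spawn zone that runs up to three waves from spawn-point arrays, with linked doors for containing the fight.
; CheckEnemyLeft advances waves at zero enemies, though wave 1 writes its count to the game mode instead.
; An empty or finished wave opens the doors and shows a win or door-unlocked widget.
; ResetSpawnzone destroys tagged enemies and restores state; the player-overlap start is disconnected.
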(event `self.ReceiveBeginPlay`
  ;[1 1 1] Sets the enemies alive to wave 1 length
)

(event `SpawnEnemy`
  (params (WaveToSpawn :type "Array of Actor Object Reference"))
  ;[1 1 1] Spawn enemies for each spawnpoint the the array in the spawnzone
  (for _array_element WaveToSpawn
    (bind _asbp_spawn_point_enemy (cast `/Game/Jeremy/Blueprints/BP_SpawnPointEnemy` _array_element))
    (`|SpawnActorFromClass` (`/Game/Jeremy/Blueprints/BP_SpawnPointEnemy.EnemyToSpawnClass` _asbp_spawn_point_enemy) (`self.GetTransform` _array_element) "AdjustIfPossibleButAlwaysSpawn" "MultiplyWithRoot" null null)))

(event `SpawnNextWave`
  (params (WaveCount :type Integer))
  (bind _wave3 (`self.Wave3`))
  (bind _wave2 (`self.Wave2`))
  (bind _wave1 (`self.Wave1`))
  ;[1 1 1] Choose what wave to spawn based on wave count.
  (switch `int` WaveCount
    (:`1`
      (`KismetSystemLibrary.PrintText` "Wave 1")
      (bind _asbp_spel_1game_mode (cast `/Game/Blueprints/BP_Spel1GameMode` (`GameplayStatics.GetGameMode`)))
      (set `/Game/Blueprints/BP_Spel1GameMode.EnemiesAlive` (`KismetArrayLibrary.Array_Length` _wave1) _asbp_spel_1game_mode)
      (`self.SpawnEnemy` _wave1))
    (:`2`
      (`KismetSystemLibrary.PrintText` "Wave 2")
      (set `self.EnemiesAliveSP` (`KismetArrayLibrary.Array_Length` _wave2))
      (if (`KismetArrayLibrary.Array_IsEmpty` _wave2)
        ;[1 1 1] When wave complete, open doors
        (`KismetSystemLibrary.PrintText` "Waves complete" :!label _label)
        (for _array_element (`self.Doors`)
          (bind _asbp_door_spawnzone (cast `/Game/Jeremy/Blueprints/BP_DoorSpawnzone` _array_element))
          (`/Game/Jeremy/Blueprints/BP_DoorSpawnzone.Open Door` _asbp_door_spawnzone)
          (if (`self.PlayerWin`)
            (`self.You Win`)
            (else
              (`self.Door Unlocked`))))
        (else
          (`self.SpawnEnemy` _wave2))))
    (:`3`
      (`KismetSystemLibrary.PrintText` "Wave 3")
      (set `self.EnemiesAliveSP` (`KismetArrayLibrary.Array_Length` _wave3))
      (if (`KismetArrayLibrary.Array_IsEmpty` _wave3)
        (goto _label)
        (else
          (`self.SpawnEnemy` _wave3))))
    (:`4`
      (goto _label))))

(event `You Win`
  ;[1 1 1] You Win Event
  (bind _returnvalue (`|CreateWidget` "/Game/Jeremy/Widgets/WBP_YouWin.WBP_YouWin_C"))
  (`UserWidget.AddToViewport` _returnvalue 0))

(event `Door Unlocked`
  ;[1 1 1] Wave Cleared Event
  (bind _returnvalue (`|CreateWidget` "/Game/Jeremy/Widgets/WBP_DoorUnlocked.WBP_DoorUnlocked_C"))
  (`UserWidget.AddToViewport` _returnvalue 0))

(event `CheckEnemyLeft`
  ;[1 1 1] Check enemy left
  (if (== (`self.EnemiesAliveSP`) 0)
    (bind _result (`/Engine/EditorBlueprintResources/StandardMacros.IncrementInt` (`self.WaveCount`))
      (:`  `
        (bind _output_get (set `self.WaveCount` _result))
        (`self.SpawnNextWave` _output_get)))))

(event `self.ReceiveActorBeginOverlap`
  (params (OtherActor :type "Actor Object Reference"))
  ;[1 1 1] If Player enters trigger, spawn first wave of enemies
)

(event `Reset Spawnzone`
  ;[1 1 1] Reset Spawnzone
  (`|ExecutionSequence`
    (:`then_0`
      ;[1 1 1] If Player enters trigger, spawn first wave of enemies
      (`/Engine/EditorBlueprintResources/StandardMacros.DoOnce` false :!via `Reset`
        (:`Completed`
          (for _array_element (`self.Doors`)
            (bind _asbp_door_spawnzone (cast `/Game/Jeremy/Blueprints/BP_DoorSpawnzone` _array_element))
            (`/Game/Jeremy/Blueprints/BP_DoorSpawnzone.Close Doors` _asbp_door_spawnzone))
          (`KismetSystemLibrary.Delay` (`self.TimeBetweenWaves`))
          (`self.SpawnNextWave` (`self.WaveCount`)))))
    (:`then_1`
      (bind _outactors (`GameplayStatics.GetAllActorsWithTag` "Enemy"))
      (for _array_element_2 _outactors
        (`self.K2_DestroyActor` _array_element_2)))
    (:`then_2`
      (set `self.WaveCount` 1)
      (for _array_element_3 (`self.Doors`)
        (bind _asbp_door_spawnzone_2 (cast `/Game/Jeremy/Blueprints/BP_DoorSpawnzone` _array_element_3))
        (`/Game/Jeremy/Blueprints/BP_DoorSpawnzone.Open Door` _asbp_door_spawnzone_2)))
    (:`then_3`
      (set `self.EnemiesAliveSP` 0))))

(fn `UserConstructionScript`)