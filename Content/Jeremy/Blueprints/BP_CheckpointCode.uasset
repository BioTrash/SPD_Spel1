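; Checkpoint actor that records a respawn point in the save game when the player overlaps its collision box.
; The overlap passes a DoOnce ahead of the player cast, then hides the checkpoint and loads the existing Save1 slot.
; It writes its own transform into BP_SaveGame's PlayerPos and saves the slot back.
; If no save exists, it only prints a message and creates none.
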(event `self.BoxCollision.OnComponentBeginOverlap`
  (params (OverlappedComponent :type "PrimitiveComponent Object Reference") (OtherActor :type "Actor Object Reference") (OtherComp :type "PrimitiveComponent Object Reference") (OtherBodyIndex :type Integer) (bFromSweep :type Boolean) (SweepResult :type "HitResult Structure (by ref)"))
  ;[1 1 1] Save Game
  (`/Engine/EditorBlueprintResources/StandardMacros.DoOnce` false
    (:`Completed`
      (cast `/Game/Blueprints/BP_PlayerCharacter` OtherActor)
      (`self.SetActorHiddenInGame` true)
      (`KismetSystemLibrary.PrintText` "Spawn point has been set")
      (bind _returnvalue (`GameplayStatics.DoesSaveGameExist` "Save1"))
      (if _returnvalue
        (bind _returnvalue_2 (`GameplayStatics.LoadGameFromSlot` "Save1"))
        (bind _asbp_save_game (cast `/Game/Jeremy/Blueprints/BP_SaveGame` _returnvalue_2))
        (set `/Game/Jeremy/Blueprints/BP_SaveGame.PlayerPos` (`self.GetTransform`) _asbp_save_game)
        (`GameplayStatics.SaveGameToSlot` _asbp_save_game "Save1")
        (`KismetSystemLibrary.PrintText` "GAME SAVED")
        (else
          (`KismetSystemLibrary.PrintText` "No save found"))))))

(fn `UserConstructionScript`)