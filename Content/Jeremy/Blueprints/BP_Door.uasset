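; Door actor that opens and closes by toggling its visibility rather than moving.
; BeginPlay hides it so it starts open; the OpenDoor event hides it and CloseDoor shows it again.
; Disconnected leftover nodes sketch an unused vertical slide based on a stored start location, move distance and direction flag, but never run.
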(event `self.ReceiveBeginPlay`
  (`self.SetActorHiddenInGame` true))

(event `self.ReceiveTick`
  (params (DeltaSeconds :type "Float (single-precision)")))

(event `Open Door`
  (`self.SetActorHiddenInGame` true))

(event `Close Door`
  (`self.SetActorHiddenInGame` false))

(fn `UserConstructionScript`)