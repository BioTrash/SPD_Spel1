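; BP_EnemyTesting is a test enemy that chases the player and has a partial death handler.
; Every Tick issues a new AI MoveTo toward the first player's pawn.
; Die only turns off physics simulation on the mesh, ignoring its Impulse input.
; The remaining death steps (mesh impulse, collision changes and the OnDeath call) are disconnected and never run.
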(event `self.ReceiveTick`
  (params (DeltaSeconds :type "Float (single-precision)"))
  ;[1 1 1] Move Toward Player
  (`|AIMoveTo` self (0.0 0.0 0.0) (`GameplayStatics.GetPlayerPawn` 0)))

(event `Die`
  (params (Impulse :type "Vector Structure"))
  ;[1 1 1] Death
  (`PrimitiveComponent.SetSimulatePhysics` (`self.Mesh`) false))

(fn `UserConstructionScript`)