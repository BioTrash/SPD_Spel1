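; BP_SecretPickup is a one-time pickup that unlocks the secret skin in the save game.
; On BeginPlay it reads save slot Save1 and destroys itself if the skin is already unlocked.
; The first player overlap with its trigger sets the unlock flag, saves the slot and destroys the pickup.
; It relies on an existing BP_SaveGame in that slot, as it never creates one.
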(event `self.ReceiveBeginPlay`
  (bind _returnvalue (`GameplayStatics.LoadGameFromSlot` "Save1"))
  (bind _asbp_save_game (cast `/Game/Jeremy/Blueprints/BP_SaveGame` _returnvalue))
  (if (`/Game/Jeremy/Blueprints/BP_SaveGame.UnlockSecretSkin` _asbp_save_game)
    (`self.K2_DestroyActor`)))

(event `self.Trigger.OnComponentBeginOverlap`
  (params (OverlappedComponent :type "PrimitiveComponent Object Reference") (OtherActor :type "Actor Object Reference") (OtherComp :type "PrimitiveComponent Object Reference") (OtherBodyIndex :type Integer) (bFromSweep :type Boolean) (SweepResult :type "HitResult Structure (by ref)"))
  (cast `/Game/Blueprints/BP_PlayerCharacter` OtherActor)
  (`/Engine/EditorBlueprintResources/StandardMacros.DoOnce` false
    (:`Completed`
      (bind _returnvalue (`GameplayStatics.LoadGameFromSlot` "Save1"))
      (bind _asbp_save_game (cast `/Game/Jeremy/Blueprints/BP_SaveGame` _returnvalue))
      (set `/Game/Jeremy/Blueprints/BP_SaveGame.UnlockSecretSkin` true _asbp_save_game)
      (`GameplayStatics.SaveGameToSlot` _asbp_save_game "Save1")
      (`self.K2_DestroyActor`))))

(fn `UserConstructionScript`)