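; BP_GoToNextLevel is a level exit that appears once the slime boss is defeated and sends the player to Whitebox_2_Test.
; BeginPlay finds BP_SlimeBossAI, and Tick polls its health, unhiding the actor and enabling the overlap trigger once at zero.
; Player overlap loads the "Save1" slot, sets new-game, room and level fields, saves to a differently named "Save" slot, then opens the level.
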(event `self.Trigger.OnComponentBeginOverlap`
  (params (OverlappedComponent :type "PrimitiveComponent Object Reference") (OtherActor :type "Actor Object Reference") (OtherComp :type "PrimitiveComponent Object Reference") (OtherBodyIndex :type Integer) (bFromSweep :type Boolean) (SweepResult :type "HitResult Structure (by ref)"))
  (cast `/Game/Blueprints/BP_PlayerCharacter` OtherActor)
  (bind _returnvalue (`GameplayStatics.LoadGameFromSlot` "Save1"))
  (bind _asbp_save_game (cast `/Game/Jeremy/Blueprints/BP_SaveGame` _returnvalue))
  (set `/Game/Jeremy/Blueprints/BP_SaveGame.IsNewGame` true _asbp_save_game)
  (set `/Game/Jeremy/Blueprints/BP_SaveGame.CurrentRoom` 1 _asbp_save_game)
  (set `/Game/Jeremy/Blueprints/BP_SaveGame.CurrentLevel` "/Game/Whitebox_2_Test.Whitebox_2_Test" _asbp_save_game)
  (`GameplayStatics.SaveGameToSlot` _asbp_save_game "Save")
  (`GameplayStatics.OpenLevelBySoftObjectPtr` "/Game/Whitebox_2_Test.Whitebox_2_Test"))

(event `self.ReceiveTick`
  (params (DeltaSeconds :type "Float (single-precision)"))
  (bind _trigger (`self.Trigger`))
  (if (<= (`SlimeBossAI.GetHealth` (`self.Boss`)) 0.0)
    (`/Engine/EditorBlueprintResources/StandardMacros.DoOnce` false
      (:`Completed`
        (`PrimitiveComponent.SetCollisionEnabled` _trigger "QueryAndPhysics")
        (`PrimitiveComponent.SetCollisionResponseToAllChannels` _trigger "ECR_Overlap")
        (`self.SetActorHiddenInGame` false)))))

(event `self.ReceiveBeginPlay`
  (bind _returnvalue (`GameplayStatics.GetActorOfClass` "/Game/AI/EnemyAI/Bosses/BossFirstLevel/BP_SlimeBossAI.BP_SlimeBossAI_C"))
  (set `self.Boss` _returnvalue))

(fn `UserConstructionScript`)