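; BP_Checkpoint is a trigger actor that saves player progress on overlap.
; A DoOnce gates the overlap ahead of the player cast, then the checkpoint hides itself for the player.
; It loads the existing BP_SaveGame from the game mode's slot, writes its own transform, the weapon's slime ammo and the controller's timer, clears the new-game flag, and saves.
; Without an existing save it only prints a message.
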(event `self.Trigger.OnComponentBeginOverlap`
  (params (OverlappedComponent :type "PrimitiveComponent Object Reference") (OtherActor :type "Actor Object Reference") (OtherComp :type "PrimitiveComponent Object Reference") (OtherBodyIndex :type Integer) (bFromSweep :type Boolean) (SweepResult :type "HitResult Structure (by ref)"))
  (bind _bp_save (`self.BP Save`))
  ;[1 1 1] Save Game
  (`/Engine/EditorBlueprintResources/StandardMacros.DoOnce` false
    (:`Completed`
      (bind _asbp_player_character (cast `/Game/Blueprints/BP_PlayerCharacter` OtherActor))
      (set `self.Player` _asbp_player_character)
      (`self.SetActorHiddenInGame` true)
      (bind _asbp_spel_1game_mode (cast `/Game/Blueprints/BP_Spel1GameMode` (`GameplayStatics.GetGameMode`)))
      (bind _output_get (set `self.Save Name` (`/Game/Blueprints/BP_Spel1GameMode.SaveName` _asbp_spel_1game_mode)))
      (bind _returnvalue (`GameplayStatics.DoesSaveGameExist` _output_get))
      (if _returnvalue
        (bind _returnvalue_2 (`GameplayStatics.LoadGameFromSlot` (`self.Save Name`)))
        (bind _asbp_save_game (cast `/Game/Jeremy/Blueprints/BP_SaveGame` _returnvalue_2))
        (bind _output_get_2 (set `self.BP Save` _asbp_save_game))
        (set `/Game/Jeremy/Blueprints/BP_SaveGame.PlayerPos` (`self.GetTransform`) _output_get_2)
        (bind _asnon_projectile_weapon (cast `NonProjectileWeapon` (`PlayerCharacter.GetTriggerWeapon` (`self.Player`))))
        (bind _asalternative_fire_mode (cast `AlternativeFireMode` _asnon_projectile_weapon))
        (set `/Game/Jeremy/Blueprints/BP_SaveGame.CurrentSlimeAmmo` (`AlternativeFireMode.GetCurrentSlimeAmmo` _asalternative_fire_mode) (`self.BP Save`))
        (set `/Game/Jeremy/Blueprints/BP_SaveGame.IsNewGame` false _bp_save)
        (bind _asspel_1player_controller (cast `Spel1PlayerController` (`GameplayStatics.GetPlayerController` 0)))
        (set `/Game/Jeremy/Blueprints/BP_SaveGame.Timer` (`Spel1PlayerController.TimePassed` _asspel_1player_controller) _bp_save)
        (`GameplayStatics.SaveGameToSlot` (`self.BP Save`) (`self.Save Name`))
        (`KismetSystemLibrary.PrintText` "GAME SAVED")
        (else
          (`KismetSystemLibrary.PrintText` "No save found"))))))

(fn `UserConstructionScript`)