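; Trigger zone that spawns up to three enemy waves, starting after a delay when the player character overlaps it.
; Each wave is an array of BP_SpawnPoint actors, each supplying the enemy class and transform to spawn.
; EnemiesCount starts at Wave 1's size and is not decremented here; at zero, Tick spawns Wave 2 once.
; Wave 3 uses the same check in a custom event that nothing here calls.
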(event `self.ReceiveBeginPlay`
  ;[1 1 1] Sets the enemies count to wave 1 length
  (set `self.EnemiesCount` (`KismetArrayLibrary.Array_Length` (`self.Wave1`))))

(event `self.ReceiveActorBeginOverlap`
  (params (OtherActor :type "Actor Object Reference"))
  ;[1 1 1] If Player enters trigger, spawn first wave of enemies
  (cast `/Game/Blueprints/BP_PlayerShooterCharacter` OtherActor)
  (`KismetSystemLibrary.Delay` (`self.TimeBetweenWaves`))
  ;[1 1 1] Spawning enemy for each spawnpoint in the array
  (for _array_element (`self.Wave1`)
    (bind _asbp_spawn_point (cast `/Game/Jeremy/Blueprints/BP_SpawnPoint` _array_element))
    (`|SpawnActorFromClass` (`/Game/Jeremy/Blueprints/BP_SpawnPoint.EnemyToSpawnClass` _asbp_spawn_point) (`self.GetTransform` _array_element) "Undefined" "MultiplyWithRoot" null null)))

(event `self.ReceiveTick`
  (params (DeltaSeconds :type "Float (single-precision)"))
  (bind _enemiescount (`self.EnemiesCount`))
  (bind _wave2 (`self.Wave2`))
  ;[1 1 1] Checks if wave 1 is dead, then resets "Enemies Count" to wave 2 length.
  (if (<= _enemiescount 0)
    (`KismetSystemLibrary.PrintText` (`KismetTextLibrary.Conv_IntToText` _enemiescount))
    (`/Engine/EditorBlueprintResources/StandardMacros.DoOnce` false
      (:`Completed`
        (`KismetSystemLibrary.Delay` (`self.TimeBetweenWaves`))
        (set `self.EnemiesCount` (`KismetArrayLibrary.Array_Length` _wave2))
        ;[1 1 1] Spawning enemy for each spawnpoint in the array
        (for _array_element _wave2
          (`KismetSystemLibrary.PrintText` "Wave 2") ; Testing
          (bind _asbp_spawn_point (cast `/Game/Jeremy/Blueprints/BP_SpawnPoint` _array_element))
          (`|SpawnActorFromClass` (`/Game/Jeremy/Blueprints/BP_SpawnPoint.EnemyToSpawnClass` _asbp_spawn_point) (`self.GetTransform` _array_element) "Undefined" "MultiplyWithRoot" null null))))))

(event `CustomEvent`
  (params (DeltaSeconds :type "Float (single-precision)"))
  (bind _wave3 (`self.Wave3`))
  ;[1 1 1] Checks if wave 2 is dead, then resets "Enemies Count" to wave 3 length.
  (if (<= (`self.EnemiesCount`) 0)
    (`/Engine/EditorBlueprintResources/StandardMacros.DoOnce` false
      (:`Completed`
        (`KismetSystemLibrary.Delay` (`self.TimeBetweenWaves`))
        (set `self.EnemiesCount` (`KismetArrayLibrary.Array_Length` _wave3))
        ;[1 1 1] Spawning enemy for each spawnpoint in the array
        (for _array_element _wave3
          (`KismetSystemLibrary.PrintText` "Wave 3") ; Testing
          (bind _asbp_spawn_point (cast `/Game/Jeremy/Blueprints/BP_SpawnPoint` _array_element))
          (`|SpawnActorFromClass` (`/Game/Jeremy/Blueprints/BP_SpawnPoint.EnemyToSpawnClass` _asbp_spawn_point) (`self.GetTransform` _array_element) "Undefined" "MultiplyWithRoot" null null))))))

(fn `UserConstructionScript`)