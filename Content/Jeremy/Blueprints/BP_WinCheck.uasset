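; BP_WinCheck is the win-condition actor that ends the game once both the slime boss and rat boss are dead.
; It caches both bosses on BeginPlay and polls their health on Tick, using a DoOnce to fade the player's music and play BossDeath audio.
; When that sound finishes, it plays BossDefeated and reverses the WBP_FadeIn animation, then opens MainMenuMap when the animation ends.
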(event `self.ReceiveBeginPlay`
  ;[1 1 1] Gets Bosses
  (bind _returnvalue (`GameplayStatics.GetActorOfClass` "/Game/AI/EnemyAI/Bosses/BossFirstLevel/BP_SlimeBossAI.BP_SlimeBossAI_C"))
  (set `self.SlimeBoss` _returnvalue)
  (bind _returnvalue_2 (`GameplayStatics.GetActorOfClass` "/Game/AI/EnemyAI/Bosses/ShooterBoss/BP_ShooterBossCharacter.BP_ShooterBossCharacter_C"))
  (set `self.RatBoss` _returnvalue_2))

(event `self.ReceiveTick`
  (params (DeltaSeconds :type "Float (single-precision)"))
  (bind _bossdeath (`self.BossDeath`))
  ;[1 1 1] Check if both bosses are dead, if so then win
  (if (and (<= (`SlimeBossAI.GetHealth` (`self.SlimeBoss`)) 0.0) (<= (`ShooterBoss.GetHealth` (`self.RatBoss`)) 0.0))
    (`/Engine/EditorBlueprintResources/StandardMacros.DoOnce` false
      (:`Completed`
        (bind _asbp_player_character (cast `/Game/Blueprints/BP_PlayerCharacter` (`GameplayStatics.GetPlayerPawn` 0)))
        (`AudioComponent.FadeOut` (`/Game/Blueprints/BP_PlayerCharacter.Music` _asbp_player_character) 10.0 0.0 "Linear")
        (if (not (and (`AudioComponent.IsPlaying` _bossdeath) (`KismetSystemLibrary.IsValid` _bossdeath)))
          (`AudioComponent.Play` _bossdeath 0.0))))))

(event `self.BossDefeated.OnAudioFinished`
  ;[1 1 1] Check if both bosses are dead, if so then win
  (`ActorComponent.K2_DestroyComponent` (`self.BossDefeated`)))

(event `self.BossDeath.OnAudioFinished`
  (bind _bossdefeated (`self.BossDefeated`))
  ;[1 1 1] Check if both bosses are dead, if so then win
  (`ActorComponent.K2_DestroyComponent` (`self.BossDeath`))
  (if (not (and (`KismetSystemLibrary.IsValid` _bossdefeated) (`AudioComponent.IsPlaying` _bossdefeated)))
    (`AudioComponent.Play` _bossdefeated 0.0)
    (bind _foundwidgets (`WidgetBlueprintLibrary.GetAllWidgetsOfClass` "/Game/UI/WBP_FadeIn.WBP_FadeIn_C" false))
    (for _array_element _foundwidgets
      (`|PlayAnimation` _array_element (`/Game/UI/WBP_FadeIn.FadeIn` _array_element) 0.0 1 "Reverse"
        (:`Finished`
          (`GameplayStatics.OpenLevel` "MainMenuMap"))))))

(fn `UserConstructionScript`)