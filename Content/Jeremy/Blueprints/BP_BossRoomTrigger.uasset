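; BP_BossRoomTrigger is a trigger volume that starts the slime boss encounter when the player enters.
; Overlap passes a DoOnce before the player cast, so any first overlapping actor consumes it.
; For the player, it closes DoorToClose, sets IsBossRoom on the game mode, activates the boss's SpawnEffect and fades in Level1Music.
; Reset reopens the DoOnce and calls ResetDoor on the door.
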(event `self.Trigger.OnComponentBeginOverlap`
  (params (OverlappedComponent :type "PrimitiveComponent Object Reference") (OtherActor :type "Actor Object Reference") (OtherComp :type "PrimitiveComponent Object Reference") (OtherBodyIndex :type Integer) (bFromSweep :type Boolean) (SweepResult :type "HitResult Structure (by ref)"))
  ;[1 1 1] Collide with player
  (`/Engine/EditorBlueprintResources/StandardMacros.DoOnce` false :!label _label
    (:`Completed`
      (cast `/Game/Blueprints/BP_PlayerCharacter` OtherActor)
      (`/Game/Jeremy/Blueprints/BP_DoorSpawnzone.Close Doors` (`self.DoorToClose`))
      (`self.Update IsBossRoom`)
      (`self.Activate Boss`)
      (bind _returnvalue (`GameplayStatics.GetActorOfClass` "/Game/Jeremy/Blueprints/BP_MusicManager.BP_MusicManager_C"))
      (bind _level1_music (`/Game/Jeremy/Blueprints/BP_MusicManager.Level1_Music` _returnvalue))
      (`AudioComponent.FadeIn` _level1_music 2.0 1.0 0.0 "Linear")
      (`AudioComponent.SetPaused` _level1_music false))))

(event `Reset`
  ;[1 1 1] Collide with player
  (`/Game/Jeremy/Blueprints/BP_DoorSpawnzone.Reset Door` (`self.DoorToClose`))
  (goto _label :!via `Reset`))

(event `Update IsBossRoom`
  ;[1 1 1] Update IsBossRoom
  (bind _asbp_spel_1game_mode (cast `/Game/Blueprints/BP_Spel1GameMode` (`GameplayStatics.GetGameMode`)))
  (set `/Game/Blueprints/BP_Spel1GameMode.isBossRoom` true _asbp_spel_1game_mode))

(event `Activate Boss`
  ;[1 1 1] Activate Boss
  (bind _returnvalue (`GameplayStatics.GetActorOfClass` "/Game/AI/EnemyAI/Bosses/BossFirstLevel/BP_SlimeBossAI.BP_SlimeBossAI_C"))
  (`ActorComponent.Activate` (`/Game/AI/EnemyAI/Bosses/BossFirstLevel/BP_SlimeBossAI.Spawn Effect` _returnvalue) false))

(fn `UserConstructionScript`)