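; Spawn zone door that slides up when a player character enters its trigger box, provided it is allowed to open.
; OpenDoor and CloseDoors events only toggle the ShouldOpen flag, which is checked on overlap begin.
; A timeline lerps the mesh's relative height, and leaving the box reverses it regardless of the flag.
; Disconnected nodes for toggling collision and visibility never run.
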(event `self.ReceiveBeginPlay`)

(event `self.Box.OnComponentEndOverlap`
  (params (OverlappedComponent :type "PrimitiveComponent Object Reference") (OtherActor :type "Actor Object Reference") (OtherComp :type "PrimitiveComponent Object Reference") (OtherBodyIndex :type Integer))
  ;[1 1 1] Close door
  (cast `/Game/Blueprints/BP_PlayerCharacter` OtherActor)
  ;[1 1 1] Open door
  (bind (_direction _open_track) (`Timeline|Open Door Timeline` :!via `Reverse` :!label _label)
    (:`Update`
      (`SceneComponent.K2_SetRelativeLocation` (`self.DoorMesh`) (`KismetMathLibrary.VLerp` (0.0 0.0 0.0) (0.0 0.0 800.0) _open_track) false false))))

(event `self.Box.OnComponentBeginOverlap`
  (params (OverlappedComponent :type "PrimitiveComponent Object Reference") (OtherActor :type "Actor Object Reference") (OtherComp :type "PrimitiveComponent Object Reference") (OtherBodyIndex :type Integer) (bFromSweep :type Boolean) (SweepResult :type "HitResult Structure (by ref)"))
  ;[1 1 1] Open door
  (if (`self.ShouldOpen`)
    (cast `/Game/Blueprints/BP_PlayerCharacter` OtherActor)
    (goto _label)))

(event `Open Door`
  ;[1 1 1] Open doors
  (set `self.ShouldOpen` true))

(event `Close Doors`
  ;[1 1 1] Close doors
  (set `self.ShouldOpen` false))

(fn `UserConstructionScript`)