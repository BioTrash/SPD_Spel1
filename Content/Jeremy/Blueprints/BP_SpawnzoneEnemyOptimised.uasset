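; Enemy spawn zone that locks the player in a room for up to three waves, then shows a win or door-unlocked widget.
; Player overlap fires once until reset, closing doors and spawning the first wave after a delay.
; The game mode's SpawnNextWave event drives later waves from spawn-point arrays, then opens doors, enables a button and unbinds.
; Binding precedes the player check, and resetting destroys every Enemy-tagged actor.
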(event `You Win`
  ;[1 1 1] You Win Event
  (bind _returnvalue (`|CreateWidget` "/Game/Jeremy/Widgets/WBP_YouWin.WBP_YouWin_C"))
  (`UserWidget.AddToViewport` _returnvalue 0))

(event `Door Unlocked`
  ;[1 1 1] Wave Cleared Event
  (bind _returnvalue (`|CreateWidget` "/Game/Jeremy/Widgets/WBP_DoorUnlocked.WBP_DoorUnlocked_C"))
  (`UserWidget.AddToViewport` _returnvalue 0))

(event `SpawnEnemiesEvent`
  (params (`Wave To Spawn` :type "Array of Actor Object Reference"))
  ;[1 1 1] Actually spawns the enemies
  (for _array_element `Wave To Spawn`
    (bind _asbp_spawn_point_enemy (cast `/Game/Jeremy/Blueprints/BP_SpawnPointEnemy` _array_element))
    (`|SpawnActorFromClass` (`/Game/Jeremy/Blueprints/BP_SpawnPointEnemy.EnemyToSpawnClass` _asbp_spawn_point_enemy) (`self.GetTransform` _array_element) "AdjustIfPossibleButAlwaysSpawn" "MultiplyWithRoot" null null)))

(event `SpawnEnemy`
  (bind _doors (`self.Doors`))
  ;[1 1 1] Spawns next wave when all enemies are dead (Jeremy)
  (switch `int` (`/Game/Blueprints/BP_Spel1GameMode.WaveCount` (stale `self.Trigger.OnComponentBeginOverlap` _asbp_spel_1game_mode))
    (:`2`
      (if (`KismetArrayLibrary.Array_IsNotEmpty` (`self.Wave2`))
        (`KismetSystemLibrary.PrintText` "Wave 2")
        (`self.SpawnEnemiesEvent` (`self.Wave2`))
        (else
          ;[1 1 1] When wave complete, open doors
          (if (`KismetArrayLibrary.Array_IsNotEmpty` _doors) :!label _label
            (for _array_element _doors
              (bind _asbp_door_spawnzone (cast `/Game/Jeremy/Blueprints/BP_DoorSpawnzone` _array_element)
                (:`then`
                  (`/Game/Jeremy/Blueprints/BP_DoorSpawnzone.Open Door` _asbp_door_spawnzone))
                (:`CastFailed`
                  _))
              (if (`self.PlayerWin`) :!label _label_2
                (`self.You Win`)
                (else
                  (`self.Door Unlocked`)))
              (set `/Game/Blueprints/BP_Spel1GameMode.WaveCount` 1 (stale `self.Trigger.OnComponentBeginOverlap` _asbp_spel_1game_mode))
              (bind _asbp_button (cast `/Game/Blueprints/BP_Button` (`self.Button`))
                (:`then`
                  (set `/Game/Blueprints/BP_Button.ShouldOpen?` true _asbp_button))
                (:`CastFailed`
                  _))
              (clear `/Game/Blueprints/BP_Spel1GameMode.SpawnNextWave` (stale `self.Trigger.OnComponentBeginOverlap` _asbp_spel_1game_mode)))
            (else
              (goto _label_2))))))
    (:`3`
      (if (`KismetArrayLibrary.Array_IsNotEmpty` (`self.Wave3`))
        (`KismetSystemLibrary.PrintText` "Wave 3")
        (`self.SpawnEnemiesEvent` (`self.Wave3`))
        (else
          (goto _label))))
    (:`4`
      (goto _label))))

(event `self.Trigger.OnComponentBeginOverlap`
  (params (OverlappedComponent :type "PrimitiveComponent Object Reference") (OtherActor :type "Actor Object Reference") (OtherComp :type "PrimitiveComponent Object Reference") (OtherBodyIndex :type Integer) (bFromSweep :type Boolean) (SweepResult :type "HitResult Structure (by ref)"))
  ;[1 1 1] Spawns wave 1 when player enters room and binds the current spawnzone to the spawn next wave event (Jeremy)
  (`|ExecutionSequence`
    (:`then_0`
      ;[1 1 1] Spawns next wave when all enemies are dead (Jeremy)
      (bind _asbp_spel_1game_mode (cast `/Game/Blueprints/BP_Spel1GameMode` (`GameplayStatics.GetGameMode`)))
      (add `/Game/Blueprints/BP_Spel1GameMode.SpawnNextWave` _asbp_spel_1game_mode (delegate `SpawnEnemy`)))
    (:`then_1`
      (cast `/Game/Blueprints/BP_PlayerCharacter` OtherActor)
      (`/Engine/EditorBlueprintResources/StandardMacros.DoOnce` false :!label _label_3
        (:`Completed`
          (for _array_element (`self.Doors`)
            (bind _asbp_door_spawnzone (cast `/Game/Jeremy/Blueprints/BP_DoorSpawnzone` _array_element))
            (`/Game/Jeremy/Blueprints/BP_DoorSpawnzone.Close Doors` _asbp_door_spawnzone))
          (`KismetSystemLibrary.Delay` (`self.TimeBetweenWaves`))
          (`GameplayStatics.PlaySound2D` "/Game/Music/SoundEffects/death_bell_sound_effect.death_bell_sound_effect" 1.0 1.0 0.0 null null)
          (`self.SpawnEnemiesEvent` (`self.Wave1`)))))))

(event `Reset Spawnzone`
  ;[1 1 1] Reset spawnzone (Jeremy)
  (`|ExecutionSequence`
    (:`then_0`
      (goto _label_3 :!via `Reset`))
    (:`then_1`
      (bind _outactors (`GameplayStatics.GetAllActorsWithTag` "Enemy"))
      (for _array_element _outactors
        (`self.K2_DestroyActor` _array_element)))))

(fn `UserConstructionScript`)